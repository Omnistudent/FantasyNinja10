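; Repeatable actor whose construction script builds instanced static mesh components from an array of entries holding mesh, material, transform and copy count.
; Each entry gets its own component with the mesh and a dynamic material instance applied.
; The copy loop body is empty: the AddInstance node meant to stack copies 100 units apart in Z is unconnected, so no instances are created.
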(event EventBeginPlay)

(event Collision|EventActorBeginOverlap
  (params (OtherActor :type Actor%20Object%20Reference)))

(event EventTick
  (params (DeltaSeconds :type Float%20%28single-precision%29)))

(fn ConstructionScript
  (for _array_element (Variables|Default|Getrepeatablesarray)
    (bind _returnvalue (AddComponent|AddInstancedStaticMeshComponent false))
    (Components|StaticMesh|SetStaticMesh _returnvalue (.staticmesh (Utilities|Struct|BreakSRepeatable _array_element)))
    (bind _returnvalue_2 (Rendering|Material|CreateDynamicMaterialInstance _returnvalue 0 (.material (Utilities|Struct|BreakSRepeatable _array_element)) "None" :!class /Script/Engine.PrimitiveComponent))
    (Rendering|Material|SetMaterial _returnvalue 0 _returnvalue_2)
    (for _index (range 0 (Variables|Default|Getcopies))
      _)))